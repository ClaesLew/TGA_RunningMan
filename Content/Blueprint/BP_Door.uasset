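; BP_Door is a sliding double door that unlocks and opens when anything overlaps its trigger.
; The Opening timeline rotates the lock, moves and shrinks the lock bar, and slides both panels apart.
; End overlap reverses the timeline, immediately for Core_PlayerCharacter and after a delay for other actors.
; A material swap on the left panel shows orange on opening and red on closing.
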(event `self.Trigger.OnComponentBeginOverlap`
  (params (OverlappedComponent :type "PrimitiveComponent Object Reference") (OtherActor :type "Actor Object Reference") (OtherComp :type "PrimitiveComponent Object Reference") (OtherBodyIndex :type Integer) (bFromSweep :type Boolean) (SweepResult :type "HitResult Structure (by ref)"))
  (`PrimitiveComponent.SetMaterial` (`self.SM_RunningAssets__DoorL`) 3 "/Game/Meshes/orange.orange")
  (bind (_direction _lockrot _lockmove _doormov) (`Timeline|Opening` :!label _label)
    (:`Update`
      (`SceneComponent.K2_SetRelativeRotation` (`self.RotAnchorLock`) (`KismetMathLibrary.RLerp` (struct) (struct :`Pitch` -70.0) _lockrot) false false)
      (`SceneComponent.K2_SetRelativeTransform` (`self.SM_RunningAssets__DooLockBar`) (`KismetMathLibrary.MakeTransform` (`KismetMathLibrary.VLerp` (0.0 0.0 0.0) (30.0 0.0 0.0) _lockmove) (struct) (`KismetMathLibrary.VLerp` (1.0 1.0 1.0) (0.5 1.0 1.0) _lockmove)) false false)
      (`SceneComponent.K2_SetRelativeLocation` (`self.SM_RunningAssets__DoorL`) (`KismetMathLibrary.VLerp` (0.0 0.0 0.0) (-180.0 0.0 0.0) _doormov) false false)
      (`SceneComponent.K2_SetRelativeLocation` (`self.SM_RunningAssets__DoorR`) (`KismetMathLibrary.VLerp` (0.0 0.0 0.0) (180.0 0.0 0.0) _doormov) false false))))

(event `self.Trigger.OnComponentEndOverlap`
  (params (OverlappedComponent :type "PrimitiveComponent Object Reference") (OtherActor :type "Actor Object Reference") (OtherComp :type "PrimitiveComponent Object Reference") (OtherBodyIndex :type Integer))
  (cast `/Game/Root_ST/Core/Framework/Core_PlayerCharacter` OtherActor
    (:`then`
      _)
    (:`CastFailed`
      (`KismetSystemLibrary.Delay` 5.0)))
  (`PrimitiveComponent.SetMaterial` (`self.SM_RunningAssets__DoorL`) 3 "/Game/Root_ST/Assets/Materials/M_BaseRed_Inst.M_BaseRed_Inst")
  (goto _label :!via `Reverse`))

(fn `UserConstructionScript`)