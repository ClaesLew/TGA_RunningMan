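; Disco ball actor that spins itself by rotating its root component on all three axes once play begins.
; The construction script caches the root's relative rotation in StartRot.
; The Disco timeline, started on BeginPlay, lerps each update from StartRot toward a fixed offset on every axis, then writes the result back to StartRot so the rotation accumulates.
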(event `self.ReceiveBeginPlay`
  (bind _startrot (`self.StartRot`))
  (bind (_direction _newtrack_0) (`Timeline|Disco`)
    (:`Update`
      (bind _returnvalue (`KismetMathLibrary.RLerp` _startrot (`KismetMathLibrary.MakeRotator` (+ (.roll _startrot) 10.0) (+ (.pitch _startrot) 10.0) (+ (.yaw _startrot) 10.0)) _newtrack_0))
      (`SceneComponent.K2_SetRelativeRotation` (`self.DefaultSceneRoot`) _returnvalue false false)
      (set `self.StartRot` _returnvalue))))

(fn `UserConstructionScript`
  (set `self.StartRot` (`SceneComponent.RelativeRotation` (`self.DefaultSceneRoot`))))