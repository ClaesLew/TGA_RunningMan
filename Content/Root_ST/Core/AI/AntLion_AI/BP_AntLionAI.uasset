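; AntLion AI character that feeds combat state to its blackboard: patrol, enemy, attacking and death.
; Sight perception filters actors by team into a hostiles list and targets the closest, storing the last seen position when sight is empty.
; Damage reduces hit points and targets the attacker, or at zero sets dead and reports a kill to the game instance.
; An attack collision toggles attacking; leaving it can trigger retargeting or idle reset.
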(event `self.ReceiveTick`
  (params (DeltaSeconds :type "Float (single-precision)"))
  ;[1 0.3877 0] DebugWidget
)

(event `self.ReceiveBeginPlay`
  ;[1 1 1] Init
  (`KismetSystemLibrary.Delay` 0.2)
  (`|ExecutionSequence`
    (:`then_0`
      (bind _output_get (set `self.ActiveBlackBoardRef` (`AIBlueprintHelperLibrary.GetBlackboard` (`self.GetController`))))
      (`BlackboardComponent.SetValueAsBool` _output_get "bStaticAI" (`self.bStaticUntilTriggered`))
      (`BlackboardComponent.SetValueAsBool` (`self.ActiveBlackBoardRef`) "bShouldPatrol" (`self.bShouldPatrol`))
      (set `self.CurrentHitPoints` (`self.MaxHitPoints`)))
    (:`then_1`
      ;[1 0.3877 0] DebugWidget
      (bind _returnvalue (`|CreateWidget` "/Game/Root_ST/Core/AI/AntLion_AI/AntlionDebugW.AntlionDebugW_C" null self))
      (`WidgetComponent.SetWidget` (`self.Widget`) _returnvalue))))

(event `self.ReceiveAnyDamage`
  (params (Damage :type "Float (single-precision)") (DamageType :type "DamageType Object Reference") (InstigatedBy :type "Controller Object Reference") (DamageCauser :type "Actor Object Reference"))
  ;[1 0.9137 0] DamageHandler
  (`self.TakeDamage` Damage)
  (if (<= (`self.CurrentHitPoints`) 0.0)
    (`PrimitiveComponent.SetCollisionEnabled` (`self.CapsuleComponent`) "NoCollision")
    (`BlackboardComponent.SetValueAsBool` (`self.ActiveBlackBoardRef`) "bDead" true)
    (bind _asbp_core_game_instance (cast `/Game/Root_ST/Core/Framework/Bp_CoreGameInstance` (`GameplayStatics.GetGameInstance`)))
    (`/Engine/EditorBlueprintResources/StandardMacros.DoOnce` false
      (:`Completed`
        (`/Game/Root_ST/Core/Framework/Bp_CoreGameInstance.OnGetKill` _asbp_core_game_instance)))
    (else
      (`/Engine/EditorBlueprintResources/StandardMacros.IsValid` DamageCauser
        (:`Is Valid`
          (bind _output_get (set `self.Enemy` DamageCauser))
          (`BlackboardComponent.SetValueAsObject` (`self.ActiveBlackBoardRef`) "CurrentEnemy" _output_get)
          (`BlackboardComponent.SetValueAsBool` (`self.ActiveBlackBoardRef`) "bEnemySpotted" true))))))

(event `self.Attackcollision.OnComponentBeginOverlap`
  (params (OverlappedComponent :type "PrimitiveComponent Object Reference") (OtherActor :type "Actor Object Reference") (OtherComp :type "PrimitiveComponent Object Reference") (OtherBodyIndex :type Integer) (bFromSweep :type Boolean) (SweepResult :type "HitResult Structure (by ref)"))
  ;[0 0.1145 1] CollisionHandler
  (if (== OtherActor (`self.Enemy`))
    (`BlackboardComponent.SetValueAsBool` (`self.ActiveBlackBoardRef`) "bIsAttacking" true)))

(event `self.Attackcollision.OnComponentEndOverlap`
  (params (OverlappedComponent :type "PrimitiveComponent Object Reference") (OtherActor :type "Actor Object Reference") (OtherComp :type "PrimitiveComponent Object Reference") (OtherBodyIndex :type Integer))
  (bind _enemy (`self.Enemy`))
  ;[0 0.1145 1] CollisionHandler
  (if (== OtherActor (`self.Enemy`))
    (`BlackboardComponent.SetValueAsBool` (`self.ActiveBlackBoardRef`) "bIsAttacking" false)
    (if (== (`GameplayStatics.GetPlayerCharacter` 0) _enemy)
      (`self.OnRecheckForMoreEnemies` :!label _label)
      (elif (`BlackboardComponent.GetValueAsBool` (`AIBlueprintHelperLibrary.GetBlackboard` _enemy) "bDead")
        (`KismetArrayLibrary.Array_RemoveItem` (`self.DetectedHostiles`) (`self.Enemy`))
        (goto _label)))))

(event `OnRecheckForMoreEnemies`
  ;[0.02238 1 0] Perception
  (`KismetSystemLibrary.Delay` 0.1)
  (if (<= (`KismetArrayLibrary.Array_LastIndex` (`self.DetectedHostiles`)) -1)
    (`self.ResetToIdle`)
    (elif (>= (`KismetArrayLibrary.Array_LastIndex` (`self.DetectedHostiles`)) 0)
      (for _array_element (`self.DetectedHostiles`)
        (`self.CheckClosestEnemy` _array_element))
      (set `self.ClosestDistance` 100000.0)
      (`BlackboardComponent.SetValueAsObject` (`self.ActiveBlackBoardRef`) "CurrentEnemy" (`self.Enemy`))
      (`BlackboardComponent.SetValueAsBool` (`self.ActiveBlackBoardRef`) "bEnemySpotted" true)
      (else
        (`self.ResetToIdle`)
        (`KismetArrayLibrary.Array_Clear` (`self.DetectedActors`))
        (`KismetArrayLibrary.Array_Clear` (`self.DetectedHostiles`))))))

(event `self.AIPerception.OnPerceptionUpdated`
  (params (UpdatedActors :type "Array of Actor Object Reference (by ref)"))
  ;[0.02238 1 0] Perception
  (for _array_element UpdatedActors
    (`KismetArrayLibrary.Array_AddUnique` (`self.DetectedActors`) _array_element)
    (if (not (`KismetArrayLibrary.Array_Contains` (`AIPerceptionComponent.GetCurrentlyPerceivedActors` (`self.AIPerception`) "/Script/AIModule.AISense_Sight") _array_element))
      (`KismetArrayLibrary.Array_RemoveItem` (`self.DetectedActors`) _array_element)))
  (if (<= (`KismetArrayLibrary.Array_LastIndex` (`AIPerceptionComponent.GetCurrentlyPerceivedActors` (`self.AIPerception`) "/Script/AIModule.AISense_Sight")) -1)
    (bind _asactor (cast `Actor` (`BlackboardComponent.GetValueAsObject` (`self.ActiveBlackBoardRef`) "CurrentEnemy")))
    (`BlackboardComponent.SetValueAsVector` (`self.ActiveBlackBoardRef`) "PlayerLastSeenPosition" (`self.K2_GetActorLocation` _asactor))
    (`BlackboardComponent.SetValueAsBool` (`self.ActiveBlackBoardRef`) "bEnemySpotted" false)
    (else
      (for _array_element_2 (`self.DetectedActors`)
        (bind _confirmedhostile (`self.CheckIfHostile` _array_element_2))
        (`/Engine/EditorBlueprintResources/StandardMacros.IsValid` _confirmedhostile
          (:`Is Valid`
            (`KismetArrayLibrary.Array_AddUnique` (`self.DetectedHostiles`) _confirmedhostile))))
      (if (>= (`KismetArrayLibrary.Array_LastIndex` (`self.DetectedHostiles`)) 0)
        (for _array_element_3 (`self.DetectedHostiles`)
          (`self.CheckClosestEnemy` _array_element_3))
        (set `self.ClosestDistance` 100000.0)
        (`BlackboardComponent.SetValueAsObject` (`self.ActiveBlackBoardRef`) "CurrentEnemy" (`self.Enemy`))
        (`BlackboardComponent.SetValueAsBool` (`self.ActiveBlackBoardRef`) "bEnemySpotted" true)
        (else
          (`self.OnRecheckForMoreEnemies`))))))

(fn `CheckClosestEnemy`
  (params (EnemyToCheck :type "Actor Object Reference"))
  (locals (ClosestDistanceX :type "Float (double-precision)" :default 100000.0))
  (bind _returnvalue (`self.GetDistanceTo` self EnemyToCheck))
  (if (< _returnvalue (`self.ClosestDistance`))
    (set `self.Enemy` EnemyToCheck)
    (set `self.ClosestDistance` _returnvalue)
    (return)))

(fn `CheckIfHostile`
  (params (FriendOrFoe :type "Actor Object Reference"))
  (returns (ConfirmedHostile :type "Actor Object Reference"))
  (bind _myteam (`self.MyTeam`))
  (bind _ascore_player_character (cast `/Game/Root_ST/Core/Framework/Core_PlayerCharacter` FriendOrFoe)
    (:`then`
      (if (== FriendOrFoe _ascore_player_character)
        (if (!= (`/Game/Root_ST/Core/Framework/Core_PlayerCharacter.PlayerTeam` _ascore_player_character) _myteam)
          (return FriendOrFoe))
        (else
          (if (!= _myteam (`BlackboardComponent.GetValueAsInt` (`AIBlueprintHelperLibrary.GetBlackboard` (`AIBlueprintHelperLibrary.GetAIController` FriendOrFoe)) "Team")) :!label _label
            (return FriendOrFoe)))))
    (:`CastFailed`
      (goto _label))))

(fn `ResetToIdle`
  (`BlackboardComponent.SetValueAsBool` (`self.ActiveBlackBoardRef`) "bIsAttacking" false)
  (`BlackboardComponent.SetValueAsBool` (`self.ActiveBlackBoardRef`) "bEnemySpotted" false)
  (`BlackboardComponent.SetValueAsBool` (`self.ActiveBlackBoardRef`) "bChasingPlayer" false)
  (`BlackboardComponent.ClearValue` (`self.ActiveBlackBoardRef`) "CurrentEnemy"))

(fn `TakeDamage`
  (params (IncomingDamage :type "Float (double-precision)"))
  (set `self.CurrentHitPoints` (- (`self.CurrentHitPoints`) IncomingDamage)))

(fn `UserConstructionScript`)