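; Enemy spawner actor that creates Ant Lion, Seeker Droid or Sniper AI pawns at its own location.
; After a delay on BeginPlay, if set to start active, OnActivateSpawner spawns either every row of a data table or one configured enemy.
; Per-type functions spawn the pawn with its team, create its default controller and copy hit points.
; Blackboard team writes are left disconnected.
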(event `self.ReceiveBeginPlay`
  (`KismetSystemLibrary.Delay` (`self.SpawnDelay`))
  (if (`self.bStartActive`)
    (`self.OnActivateSpawner`)))

(event `OnActivateSpawner`
  (bind _singleenemystats (`self.SingleEnemyStats`))
  (bind _spawnlist (`self.SpawnList`))
  (if (`self.bSpawnFromDataTable`)
    (bind _outrownames (`DataTableFunctionLibrary.GetDataTableRowNames` _spawnlist))
    (for _array_element _outrownames
      (bind _returnvalue (`|GetDataTableRow` _spawnlist _array_element)
        (:`then`
          (switch `/Game/Root_ST/Core/AI/EnemyTypes` (`.EnemyType_2_5615A5F9432B648A80987CB223FAB2B7` (break `/Game/Root_ST/Core/AI/EnemyStats` _returnvalue))
            (:`NewEnumerator0`
              (`self.SpawnAntLion` _returnvalue))
            (:`NewEnumerator1`
              (`self.SpawnSeekerDroid` _returnvalue))
            (:`NewEnumerator2`
              (`self.SpawnSniper` _returnvalue))))
        (:`RowNotFound`
          (`KismetSystemLibrary.PrintString` "Row not found"))))
    (`KismetSystemLibrary.PrintString` "spawn complete")
    (else
      (switch `/Game/Root_ST/Core/AI/EnemyTypes` (`.EnemyType_2_5615A5F9432B648A80987CB223FAB2B7` (break `/Game/Root_ST/Core/AI/EnemyStats` (`self.SingleEnemyStats`)))
        (:`NewEnumerator0`
          (`self.SpawnAntLion` _singleenemystats))
        (:`NewEnumerator1`
          (`self.SpawnSeekerDroid` _singleenemystats))
        (:`NewEnumerator2`
          (`self.SpawnSniper` _singleenemystats))))))

(fn `SpawnAntLion`
  (params (DataTableRow :type "/Game/Root_ST/Core/AI/EnemyStats Structure"))
  (bind (_enemytype _maxhitpoints _currenthitpoints _team) (break `/Game/Root_ST/Core/AI/EnemyStats` DataTableRow))
  (bind _returnvalue (`|SpawnActorFromClass` "/Game/Root_ST/Core/AI/AntLion_AI/BP_AntLionAI.BP_AntLionAI_C" (`SceneComponent.K2_GetComponentToWorld` (`self.DefaultSceneRoot`)) "AdjustIfPossibleButAlwaysSpawn" "OverrideRootScale" null false _team false null false null))
  (`Pawn.SpawnDefaultController` _returnvalue)
  (`|ExecutionSequence`
    (:`then_0`
      (set `/Game/Root_ST/Core/AI/AntLion_AI/BP_AntLionAI.MaxHitPoints` _maxhitpoints _returnvalue))
    (:`then_1`
      (set `/Game/Root_ST/Core/AI/AntLion_AI/BP_AntLionAI.CurrentHitPoints` _currenthitpoints _returnvalue))))

(fn `SpawnSeekerDroid`
  (params (DataTableRow :type "/Game/Root_ST/Core/AI/EnemyStats Structure"))
  (bind (_enemytype _maxhitpoints _currenthitpoints _team) (break `/Game/Root_ST/Core/AI/EnemyStats` DataTableRow))
  (bind _returnvalue (`|SpawnActorFromClass` "/Game/Root_ST/Core/AI/SeekerDroid_AI/BP_SeekerDroidAI.BP_SeekerDroidAI_C" (`KismetMathLibrary.MakeTransform` (`SceneComponent.K2_GetComponentLocation` (`self.DefaultSceneRoot`))) "AdjustIfPossibleButAlwaysSpawn" "OverrideRootScale" null false 50.0 _team null))
  (`Pawn.SpawnDefaultController` _returnvalue)
  (`|ExecutionSequence`
    (:`then_0`
      (set `/Game/Root_ST/Core/AI/SeekerDroid_AI/BP_SeekerDroidAI.HitPoints` _maxhitpoints _returnvalue))
    (:`then_1`
      (set `/Game/Root_ST/Core/AI/SeekerDroid_AI/BP_SeekerDroidAI.CurrentHitPoints` _currenthitpoints _returnvalue))))

(fn `SpawnSniper`
  (params (DataTableRow :type "/Game/Root_ST/Core/AI/EnemyStats Structure"))
  (bind (_enemytype _maxhitpoints _currenthitpoints _team) (break `/Game/Root_ST/Core/AI/EnemyStats` DataTableRow))
  (bind _returnvalue (`|SpawnActorFromClass` "/Game/Root_ST/Core/AI/Sniper_AI/BP_SniperAI.BP_SniperAI_C" (`SceneComponent.K2_GetComponentToWorld` (`self.DefaultSceneRoot`)) "AdjustIfPossibleButAlwaysSpawn" "OverrideRootScale" null false _team null))
  (`Pawn.SpawnDefaultController` _returnvalue)
  (`|ExecutionSequence`
    (:`then_0`
      (set `/Game/Root_ST/Core/AI/Sniper_AI/BP_SniperAI.MaxHitPoints` _maxhitpoints _returnvalue))
    (:`then_1`
      (set `/Game/Root_ST/Core/AI/Sniper_AI/BP_SniperAI.CurrentHitPoints` _currenthitpoints _returnvalue))))

(fn `UserConstructionScript`)