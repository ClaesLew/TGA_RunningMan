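; BP_PatrolPoint is an AI patrol waypoint actor that links to a following point through NextPatrolPoint.
; Its Construction Script labels the TextRender with the actor's display name and, when ShowpatrolPaths is on, draws a long-lived debug line to the next valid point.
; Each construction run first flushes all persistent debug lines, including those drawn by other points.
; The event graph holds no active logic.
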(fn `UserConstructionScript`
  (`TextRenderComponent.K2_SetText` (`self.TextRender`) (`KismetTextLibrary.Conv_StringToText` (`KismetSystemLibrary.GetDisplayName` self)))
  (`KismetSystemLibrary.FlushPersistentDebugLines`)
  (if (`self.bShowpatrolPaths`)
    (`self.NextPatrolPoint`
      (:`then`
        (`KismetSystemLibrary.DrawDebugLine` (`self.K2_GetActorLocation`) (`self.K2_GetActorLocation` (`self.NextPatrolPoint`)) (struct :`R` 1.0 :`G` 0.038484 :`A` 1.0) 9999.0 10.0))
      (:`else`))))