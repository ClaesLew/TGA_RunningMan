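; Seeker droid AI actor that detects, tracks and attacks hostiles, driving its behavior through blackboard keys.
; Perception updates filter actors by team, pick the closest enemy and record its last seen position when lost.
; Damage lowers hit points, retargets to the causer, or flags death and reports a kill to the game instance.
; Enemy overlap sets the attacking flag, but its end-overlap reset is disconnected; Tick nudges the mesh upward for wobble.
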(event `self.ReceiveTick`
  (params (DeltaSeconds :type "Float (single-precision)"))
  (bind (_relativelocation_x _relativelocation_y _relativelocation_z) (`KismetMathLibrary.BreakVector` (`SceneComponent.RelativeLocation` (`self.Mesh`))))
  (if (not (> (`self.WobbleHeight`) (`self.WobbleMax`)))
    (`/Engine/EditorBlueprintResources/StandardMacros.FlipFlop`
      (:`A`
        (`/Engine/EditorBlueprintResources/StandardMacros.IncrementFloat` (`self.WobbleHeight`)
          (:`  `
            (`SceneComponent.K2_SetRelativeLocation` (`self.Mesh`) (`KismetMathLibrary.MakeVector` _relativelocation_x _relativelocation_y (+ _relativelocation_z (`self.WobbleHeight`))) false false)))))))

(event `self.ReceiveBeginPlay`
  ;[1 1 1] Init
  (`KismetSystemLibrary.Delay` 0.2)
  (bind _output_get (set `self.ActiveBlackBoardRef` (`AIBlueprintHelperLibrary.GetBlackboard` (`self.GetController`))))
  (`BlackboardComponent.SetValueAsBool` _output_get "bStaticAI" (`self.bStaticUntilActive`))
  (`BlackboardComponent.SetValueAsBool` _output_get "bShouldPatrol" (`self.bShouldPatrol`))
  (set `self.CurrentHitPoints` (`self.HitPoints`)))

(event `self.AIPerception.OnPerceptionUpdated`
  (params (UpdatedActors :type "Array of Actor Object Reference (by ref)"))
  ;[0.01569 1 0] Ai Perception
  (`KismetArrayLibrary.Array_Clear` (`self.DetectedActors`))
  (`KismetArrayLibrary.Array_Clear` (`self.DetectedHostiles`))
  (bind _output_get (set `self.DetectedActors` UpdatedActors))
  (if (<= (`KismetArrayLibrary.Array_LastIndex` (`AIPerceptionComponent.GetCurrentlyPerceivedActors` (`self.AIPerception`) "/Script/AIModule.AISense_Sight")) -1)
    (bind _asactor (cast `Actor` (`BlackboardComponent.GetValueAsObject` (`self.ActiveBlackBoardRef`) "CurrentEnemy")))
    (`BlackboardComponent.SetValueAsVector` (`self.ActiveBlackBoardRef`) "PlayerLastSeenPosition" (`self.K2_GetActorLocation` _asactor))
    (`BlackboardComponent.SetValueAsBool` (`self.ActiveBlackBoardRef`) "bEnemySpotted" false)
    (else
      (for _array_element _output_get
        (bind _confirmedhostile (`self.CheckIfHostile` _array_element))
        (`/Engine/EditorBlueprintResources/StandardMacros.IsValid` _confirmedhostile
          (:`Is Valid`
            (`KismetArrayLibrary.Array_Add` (`self.DetectedHostiles`) _confirmedhostile))))
      (if (>= (`KismetArrayLibrary.Array_LastIndex` (`self.DetectedHostiles`)) 0)
        (for _array_element_2 (`self.DetectedHostiles`)
          (`self.CheckClosestEnemy` _array_element_2)
          (bind _enemy (`self.Enemy`)
            (:`then`
              (`BlackboardComponent.SetValueAsObject` (`self.ActiveBlackBoardRef`) "CurrentEnemy" _enemy)
              (`BlackboardComponent.SetValueAsBool` (`self.ActiveBlackBoardRef`) "bEnemySpotted" true))
            (:`else`)))
        (else
          (`self.Enemy`
            (:`then`
              (bind _asactor_2 (cast `Actor` (`BlackboardComponent.GetValueAsObject` (`self.ActiveBlackBoardRef`) "CurrentEnemy")))
              (`BlackboardComponent.SetValueAsVector` (`self.ActiveBlackBoardRef`) "PlayerLastSeenPosition" (`self.K2_GetActorLocation` _asactor_2))
              (`BlackboardComponent.SetValueAsBool` (`self.ActiveBlackBoardRef`) "bEnemySpotted" false))
            (:`else`)))))))

(event `self.ReceiveAnyDamage`
  (params (Damage :type "Float (single-precision)") (DamageType :type "DamageType Object Reference") (InstigatedBy :type "Controller Object Reference") (DamageCauser :type "Actor Object Reference"))
  ;[1 0.9137 0] DamageHandling
  (`self.TakeDamage` Damage)
  (if (<= (`self.CurrentHitPoints`) 0.0)
    (`BlackboardComponent.SetValueAsBool` (`self.ActiveBlackBoardRef`) "bDead" true)
    (bind _asbp_core_game_instance (cast `/Game/Root_ST/Core/Framework/Bp_CoreGameInstance` (`GameplayStatics.GetGameInstance`)))
    (`/Engine/EditorBlueprintResources/StandardMacros.DoOnce` false
      (:`Completed`
        (`/Game/Root_ST/Core/Framework/Bp_CoreGameInstance.OnGetKill` _asbp_core_game_instance)))
    (else
      (`/Engine/EditorBlueprintResources/StandardMacros.IsValid` DamageCauser
        (:`Is Valid`
          (set `self.Enemy` DamageCauser)
          (`BlackboardComponent.SetValueAsObject` (`self.ActiveBlackBoardRef`) "CurrentEnemy" DamageCauser)
          (`BlackboardComponent.SetValueAsBool` (`self.ActiveBlackBoardRef`) "bEnemySpotted" true))))))

(event `self.Attackcollision.OnComponentBeginOverlap`
  (params (OverlappedComponent :type "PrimitiveComponent Object Reference") (OtherActor :type "Actor Object Reference") (OtherComp :type "PrimitiveComponent Object Reference") (OtherBodyIndex :type Integer) (bFromSweep :type Boolean) (SweepResult :type "HitResult Structure (by ref)"))
  ;[0 0.1137 1] CollisionHandling
  (if (== OtherActor (`self.Enemy`))
    (`BlackboardComponent.SetValueAsBool` (`self.ActiveBlackBoardRef`) "bIsAttacking" true)))

(event `self.Attackcollision.OnComponentEndOverlap`
  (params (OverlappedComponent :type "PrimitiveComponent Object Reference") (OtherActor :type "Actor Object Reference") (OtherComp :type "PrimitiveComponent Object Reference") (OtherBodyIndex :type Integer))
  ;[0 0.1137 1] CollisionHandling
)

(fn `CheckClosestEnemy`
  (params (SpottedEnemy :type "Actor Object Reference"))
  (locals (ClosestDistance :type "Float (double-precision)" :default 100000.0))
  (bind _returnvalue (`self.GetDistanceTo` self SpottedEnemy))
  (if (< _returnvalue (`local.ClosestDistance`))
    (set `self.Enemy` SpottedEnemy)
    (set `local.ClosestDistance` _returnvalue)))

(fn `CheckIfHostile`
  (params (FirendOrFoe :type "Actor Object Reference"))
  (returns (ConfirmedHostile :type "Actor Object Reference"))
  (bind _myteam (`self.MyTeam`))
  (bind _ascore_player_character (cast `/Game/Root_ST/Core/Framework/Core_PlayerCharacter` FirendOrFoe)
    (:`then`
      (if (== FirendOrFoe _ascore_player_character)
        (if (!= (`/Game/Root_ST/Core/Framework/Core_PlayerCharacter.PlayerTeam` _ascore_player_character) _myteam)
          (return FirendOrFoe))
        (else
          (if (!= _myteam (`BlackboardComponent.GetValueAsInt` (`AIBlueprintHelperLibrary.GetBlackboard` (`AIBlueprintHelperLibrary.GetAIController` FirendOrFoe)) "Team")) :!label _label
            (return FirendOrFoe)))))
    (:`CastFailed`
      (goto _label))))

(fn `TakeDamage`
  (params (IncomingDamage :type "Float (double-precision)"))
  (set `self.CurrentHitPoints` (- (`self.CurrentHitPoints`) IncomingDamage)))

(fn `UserConstructionScript`)