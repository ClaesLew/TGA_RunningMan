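; Sniper AI character that spots hostiles, tracks them with a laser sight and fires hitscan shots.
; Sight perception filters actors by team and writes the nearest enemy to the Blackboard; damage also sets the attacker as enemy or flags death.
; OnSniperAim eases aim pitch and yaw onto the target via a timeline, fires if still aiming, then rechecks for enemies.
; A line trace updates the laser endpoint each tick.
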(event `self.ReceiveBeginPlay`
  (bind _mesh (`self.Mesh`))
  (if (not (`self.bIsCutscene`))
    (`AIPerceptionComponent.SetSenseEnabled` (`self.AIPerception`) "/Script/AIModule.AISense_Sight" false)
    ;[1 1 1] Init
    (set `SkeletalMeshComponent.bPauseAnims` true _mesh)
    (`KismetSystemLibrary.Delay` (`KismetMathLibrary.RandomFloatInRange` 0.2 0.4))
    (set `SkeletalMeshComponent.bPauseAnims` false _mesh)
    (bind _output_get (set `self.ActiveBlackBoardRef` (`AIBlueprintHelperLibrary.GetBlackboard` (`self.GetController`))))
    (`BlackboardComponent.SetValueAsBool` _output_get "bStaticAI" (`self.bStaticUntilTriggered`))
    (set `self.CurrentHitPoints` (`self.MaxHitPoints`))
    (set `self.PreviousPitchPos` 0.0)
    (set `self.PreviousYawPos` 0.0)
    (set `self.bIsCrouching` false)))

(event `OnSniperAim`
  ;[0 0.4873 1] Shooting
  (if (not (`self.bIsFocusing`))
    (`self.Enemy`
      (:`then`
        (`|ExecutionSequence`
          (:`then_0`
            (`self.SetAimOffsetpoint`))
          (:`then_1`
            (set `self.bIsFocusing` true)
            (`self.OnFocusTrackerBeam`))))
      (:`else`))))

(event `OnFocusTrackerBeam`
  (bind _previousyawpos (`self.PreviousYawPos`))
  ;[0 0.4873 1] Shooting
  (bind (_direction _focus_on_player) (`Timeline|TrackerTime` :!via `PlayFromStart`)
    (:`Update`
      (set `self.AimYaw` (`KismetMathLibrary.Lerp` (`self.PreviousYawPos`) (`self.YawRef`) _focus_on_player))
      (set `self.AimPitch` (`KismetMathLibrary.Lerp` (`self.PreviousPitchPos`) (`self.PitchRef`) _focus_on_player)))
    (:`Finished`
      (set `self.PreviousPitchPos` (`self.PitchRef`))
      (set `self.PreviousYawPos` (`self.YawRef`))
      (if (`BlackboardComponent.GetValueAsBool` (`self.ActiveBlackBoardRef`) "bAiming")
        (`self.OnShoot`)
        (else
          (`/Engine/EditorBlueprintResources/StandardMacros.FlipFlop`
            (:`A`
              (set `self.PreviousYawPos` (* _previousyawpos -1.0)))
            (:`B`
              (set `self.PreviousYawPos` _previousyawpos))))))))

(event `self.ReceiveAnyDamage`
  (params (Damage :type "Float (single-precision)") (DamageType :type "DamageType Object Reference") (InstigatedBy :type "Controller Object Reference") (DamageCauser :type "Actor Object Reference"))
  (bind _activeblackboardref (`self.ActiveBlackBoardRef`))
  ;[1 0.9124 0] DamageHandling
  (`self.TakeDamage` Damage)
  (if (<= (`self.CurrentHitPoints`) 0.0)
    (`BlackboardComponent.SetValueAsBool` _activeblackboardref "bDead" true)
    (`PrimitiveComponent.SetCollisionEnabled` (`self.CapsuleComponent`) "NoCollision")
    (bind _asbp_core_game_instance (cast `/Game/Root_ST/Core/Framework/Bp_CoreGameInstance` (`GameplayStatics.GetGameInstance`)))
    (`/Engine/EditorBlueprintResources/StandardMacros.DoOnce` false
      (:`Completed`
        (`/Game/Root_ST/Core/Framework/Bp_CoreGameInstance.OnGetKill` _asbp_core_game_instance)))
    (else
      (`/Engine/EditorBlueprintResources/StandardMacros.IsValid` DamageCauser
        (:`Is Valid`
          (bind _output_get (set `self.Enemy` DamageCauser))
          (`BlackboardComponent.SetValueAsObject` _activeblackboardref "CurrentEnemy" _output_get))))))

(event `self.ReceiveTick`
  (params (DeltaSeconds :type "Float (single-precision)"))
  ;[0 0.4873 1] Shooting
  (`self.SetBeamEnd`))

(event `OnShoot`
  (bind _beampoint (`self.Beampoint`))
  ;[0 0.4873 1] Shooting
  (if (`BlackboardComponent.GetValueAsBool` (`self.ActiveBlackBoardRef`) "bDead")
    (`KismetSystemLibrary.PrintString` "NO SHOT SINCE IM DEAD" true true (struct :`R` 1.0 :`B` 0.00845 :`A` 1.0) 20.0)
    (else
      (set `self.bIsShooting` true)
      (`GameplayStatics.SpawnEmitterAttached` "/Game/Root_ST/Assets/WeaponsAndPickups/Fal/Materials/Muzzleflare/P_Muzzle1.P_Muzzle1" (`self.SkeletalMesh`) "MuzzleFlashSocket")
      (bind _outhit (`KismetSystemLibrary.LineTraceSingle` :`Start` (`SceneComponent.K2_GetComponentLocation` (`self.Beampoint`)) :`End` (+ (`SceneComponent.K2_GetComponentLocation` _beampoint) (* (`SceneComponent.GetForwardVector` _beampoint) 5000.0)) :`TraceChannel` "TraceTypeQuery2" :`bTraceComplex` true :`DrawDebugType` "ForOneFrame" :`TraceColor` (struct :`R` 0.018122 :`G` 0.20024 :`B` 1.0 :`A` 1.0) :`DrawTime` 10.0))
      (bind (_bblockinghit _binitialoverlap _time _distance _location _impactpoint _normal _impactnormal _physmat _hitactor) (`GameplayStatics.BreakHitResult` _outhit))
      (`GameplayStatics.SpawnEmitterAtLocation` "/Game/Root_ST/Assets/FX/Particles/P_BulletExplosion.P_BulletExplosion" _impactpoint (struct) (0.3 0.3 0.3))
      (`GameplayStatics.PlaySoundAtLocation` "/Game/StarterContent/Audio/Explosion_Cue.Explosion_Cue" _impactpoint (struct) 1.0 1.0 0.0 null null null)
      (`GameplayStatics.ApplyDamage` _hitactor (`self.Damage`) null self)
      (`KismetSystemLibrary.Delay` (`KismetMathLibrary.RandomFloatInRange` 1.1 1.5))
      (set `self.bIsShooting` false)
      (set `self.bIsFocusing` false)
      (`self.OnRecheckForMoreEnemies`))))

(event `OnRecheckForMoreEnemies`
  (bind _outactors (`AIPerceptionComponent.GetCurrentlyPerceivedActors` (`self.AIPerception`) "/Script/AIModule.AISense_Sight"))
  ;[0.01569 1 0] LookForNewEnemies
  (`KismetSystemLibrary.Delay` 1.0)
  (`KismetArrayLibrary.Array_Clear` (`self.DetectedActors`))
  (`KismetArrayLibrary.Array_Clear` (`self.DetectedHostiles`))
  (if (<= (`KismetArrayLibrary.Array_LastIndex` _outactors) -1)
    (`BlackboardComponent.SetValueAsBool` (`self.ActiveBlackBoardRef`) "bEnemySpotted" false)
    (`BlackboardComponent.ClearValue` (`self.ActiveBlackBoardRef`) "CurrentEnemy")
    (else
      (for _array_element _outactors
        (bind _asai_master_controller (cast `/Game/Root_ST/Core/AI/AI_MasterController` (`AIBlueprintHelperLibrary.GetAIController` _array_element))
          (:`then`
            (if (`/Game/Root_ST/Core/AI/AI_MasterController.bSetupCompleted` _asai_master_controller)
              (bind _confirmedenemy (`self.CheckIfHostile` _array_element :!label _label))
              (`/Engine/EditorBlueprintResources/StandardMacros.IsValid` _confirmedenemy
                (:`Is Valid`
                  (`KismetArrayLibrary.Array_AddUnique` (`self.DetectedHostiles`) _confirmedenemy)))))
          (:`CastFailed`
            (goto _label))))
      ;;[1 0.03471 0] Same here - Go find!
      (bind _closestenemy (`self.CheckClosestEnemy` null (`self.DetectedHostiles`)))
      (bind _output_get (set `self.Enemy` _closestenemy))
      (`BlackboardComponent.SetValueAsObject` (`self.ActiveBlackBoardRef`) "CurrentEnemy" _output_get)
      (`BlackboardComponent.SetValueAsBool` (`self.ActiveBlackBoardRef`) "bEnemySpotted" true))))

(event `self.AIPerception.OnPerceptionUpdated`
  (params (UpdatedActors :type "Array of Actor Object Reference (by ref)"))
  ;[0.01569 1 0] Perception
  (if true
    (`KismetArrayLibrary.Array_Clear` (`self.DetectedActors`))
    (`KismetArrayLibrary.Array_Clear` (`self.DetectedHostiles`))
    (bind _output_get (set `self.DetectedActors` (`AIPerceptionComponent.GetCurrentlyPerceivedActors` (`self.AIPerception`) "/Script/AIModule.AISense_Sight")))
    (for _array_element _output_get
      (bind _asai_master_controller (cast `/Game/Root_ST/Core/AI/AI_MasterController` (`AIBlueprintHelperLibrary.GetAIController` _array_element))
        (:`then`
          (if (`/Game/Root_ST/Core/AI/AI_MasterController.bSetupCompleted` _asai_master_controller)
            (bind _confirmedenemy (`self.CheckIfHostile` _array_element :!label _label_2))
            (`/Engine/EditorBlueprintResources/StandardMacros.IsValid` _confirmedenemy
              (:`Is Valid`
                (`KismetArrayLibrary.Array_AddUnique` (`self.DetectedHostiles`) _confirmedenemy)))))
        (:`CastFailed`
          (goto _label_2))))
    (if (>= (`KismetArrayLibrary.Array_LastIndex` (`self.DetectedHostiles`)) 0)
      ;;[1 0 0.01447] This Function will not work - Why?
      (bind _closestenemy (`self.CheckClosestEnemy` null (`self.DetectedHostiles`)))
      (bind _output_get_2 (set `self.Enemy` _closestenemy))
      (`BlackboardComponent.SetValueAsObject` (`self.ActiveBlackBoardRef`) "CurrentEnemy" _output_get_2)
      (`BlackboardComponent.SetValueAsBool` (`self.ActiveBlackBoardRef`) "bEnemySpotted" true))))

(event `self.AIPerception.OnTargetPerceptionUpdated`
  (params (Actor :type "Actor Object Reference") (Stimulus :type "AIStimulus Structure"))
  ;[1 0.1144 0] Junk Perception
)

(fn `AngleOfVectors`
  (params (Vector1 :type "Vector Structure") (Vector2 :type "Vector Structure"))
  (returns (Degrees :type "Float (double-precision)"))
  (return (`KismetMathLibrary.DegAcos` (`KismetMathLibrary.Dot_VectorVector` (`KismetMathLibrary.Normal` Vector1) (`KismetMathLibrary.Normal` Vector2)))))

(fn `CheckClosestEnemy`
  (params (SpottedEnemy :type "Actor Object Reference") (DetectedEnemies :type "Array of Actor Object Reference"))
  (returns (ClosestEnemy :type "Actor Object Reference"))
  (locals (ClosestDistance :type "Float (double-precision)" :default 10000.0))
  (for _array_element DetectedEnemies
    (bind _returnvalue (`self.GetDistanceTo` self _array_element))
    (if (< _returnvalue (`local.ClosestDistance`))
      (set `self.Enemy` _array_element)
      (set `local.ClosestDistance` _returnvalue)))
  (set `local.ClosestDistance` 10000.0)
  (return (`self.Enemy`)))

(fn `CheckIfHostile`
  (params (FirendOrFoe :type "Actor Object Reference"))
  (returns (ConfirmedEnemy :type "Actor Object Reference"))
  (bind _myteam (`self.MyTeam`))
  (bind _ascore_player_character (cast `/Game/Root_ST/Core/Framework/Core_PlayerCharacter` FirendOrFoe)
    (:`then`
      (if (== FirendOrFoe _ascore_player_character)
        (if (!= (`/Game/Root_ST/Core/Framework/Core_PlayerCharacter.PlayerTeam` _ascore_player_character) _myteam)
          (return FirendOrFoe))
        (else
          (if (!= _myteam (`BlackboardComponent.GetValueAsInt` (`AIBlueprintHelperLibrary.GetBlackboard` (`AIBlueprintHelperLibrary.GetAIController` FirendOrFoe)) "Team")) :!label _label
            (return FirendOrFoe)))))
    (:`CastFailed`
      (goto _label))))

(fn `SetAimOffsetpoint`
  (bind _returnvalue (`self.K2_GetActorLocation` self))
  (bind _returnvalue_2 (+ (`self.K2_GetActorLocation` (`self.Enemy`)) (0.0 0.0 75.0)))
  (set `self.PitchRef` (.pitch (`KismetMathLibrary.FindLookAtRotation` _returnvalue _returnvalue_2)))
  (set `self.YawRef` (* (.yaw (`KismetMathLibrary.NormalizedDeltaRotator` (`self.K2_GetActorRotation`) (`KismetMathLibrary.MakeRotFromX` (- _returnvalue_2 _returnvalue)))) -1.0))
  (return))

(fn `SetBeamEnd`
  (bind _beampoint (`self.Beampoint`))
  (bind _p_laserbeam (`self.P_LaserBeam`))
  (bind (_outhit _returnvalue) (`KismetSystemLibrary.LineTraceSingle` :`Start` (`SceneComponent.K2_GetComponentLocation` (`self.Beampoint`)) :`End` (+ (`SceneComponent.K2_GetComponentLocation` _beampoint) (* (`SceneComponent.GetForwardVector` _beampoint) 5000.0)) :`TraceChannel` "TraceTypeQuery2" :`bTraceComplex` true :`TraceColor` (struct :`R` 1.0 :`G` 0.818537 :`A` 1.0) :`DrawTime` 1.0))
  (if _returnvalue
    (bind (_bblockinghit _binitialoverlap _time _distance _location _impactpoint _normal _impactnormal _physmat _hitactor _hitcomponent _hitbonename _hititem _faceindex _tracestart _traceend) (`GameplayStatics.BreakHitResult` _outhit))
    (`ParticleSystemComponent.SetBeamTargetPoint` _p_laserbeam 0 _location 0)
    (else
      (`ParticleSystemComponent.SetBeamTargetPoint` _p_laserbeam 0 _traceend 0)))
  (return))

(fn `TakeDamage`
  (params (IncomingDamage :type "Float (double-precision)"))
  (set `self.CurrentHitPoints` (- (`self.CurrentHitPoints`) IncomingDamage)))

(fn `UserConstructionScript`
  (bind _beampoint (`self.Beampoint`))
  (bind _p_laserbeam (`self.P_LaserBeam`))
  (bind (_outhit _returnvalue) (`KismetSystemLibrary.LineTraceSingle` :`Start` (`SceneComponent.K2_GetComponentLocation` (`self.Beampoint`)) :`End` (+ (`SceneComponent.K2_GetComponentLocation` _beampoint) (* (`SceneComponent.GetForwardVector` _beampoint) 5000.0)) :`TraceChannel` "TraceTypeQuery2" :`bTraceComplex` true :`TraceColor` (struct :`R` 1.0 :`G` 0.818537 :`A` 1.0) :`DrawTime` 1.0))
  (if _returnvalue
    (bind (_bblockinghit _binitialoverlap _time _distance _location _impactpoint _normal _impactnormal _physmat _hitactor _hitcomponent _hitbonename _hititem _faceindex _tracestart _traceend) (`GameplayStatics.BreakHitResult` _outhit))
    (`ParticleSystemComponent.SetBeamTargetPoint` _p_laserbeam 0 _location 0)
    (else
      (`ParticleSystemComponent.SetBeamTargetPoint` _p_laserbeam 0 _traceend 0))))